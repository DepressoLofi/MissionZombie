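; BP_Zachary is a player-controlled pawn with Enhanced Input movement.
; On BeginPlay it casts its controller to BP_ZacController and adds the IMC_Zac mapping context to that player's input subsystem.
; IA_ZacMove feeds X and Y into movement input along the control rotation's right and forward vectors, with pitch zeroed for the forward direction and for the right.
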(event `self.ReceiveBeginPlay`
  ;[1 0.7291 0.6912] Control setup
  (bind _asbp_zac_controller (cast `/Game/Blueprints/BP_ZacController` (`self.GetController`)))
  (`EnhancedInputSubsystemInterface.AddMappingContext` (pcsubsystem `EnhancedInputLocalPlayerSubsystem` _asbp_zac_controller) "/Game/Inputs/IMC_Zac.IMC_Zac" 0 (struct)))

(event `EnhancedInput|/Game/Inputs/IA_ZacMove`
  (params (ActionValue :type "Vector2D Structure") (ElapsedSeconds :type "Float (double-precision)") (TriggeredSeconds :type "Float (double-precision)") (InputAction :type "InputAction Object Reference" :default "/Game/Inputs/IA_ZacMove.IA_ZacMove"))
  (bind (_returnvalue_roll _returnvalue_pitch _returnvalue_yaw) (`KismetMathLibrary.BreakRotator` (`self.GetControlRotation`)))
  (bind (_returnvalue_roll_2 _returnvalue_pitch_2 _returnvalue_yaw_2) (`KismetMathLibrary.BreakRotator` (`self.GetControlRotation`)))
  (:`Triggered`
    (`self.AddMovementInput` (`KismetMathLibrary.GetRightVector` (`KismetMathLibrary.MakeRotator` _returnvalue_roll 0.0 _returnvalue_yaw)) ActionValue_X)
    (`self.AddMovementInput` (`KismetMathLibrary.GetForwardVector` (`KismetMathLibrary.MakeRotator` _returnvalue_roll_2 0.0 _returnvalue_yaw_2)) ActionValue_Y)))

(fn `UserConstructionScript`)